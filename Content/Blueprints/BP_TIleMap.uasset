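; Tile map actor that builds the game board as a grid of BP_Tile actors and registers itself with BP_GameInstance.
; On BeginPlay, BuildBoard spawns and attaches tiles around a center point, then each tile's neighbors are cached through eight line traces in straight and diagonal directions.
; It then spawns an object spawner and tells it to spawn objects.
; An index-based neighbor lookup, PopulateAdjacentTiles, is defined but not called here.
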(event `self.ReceiveBeginPlay`
  (bind _asbp_game_instance (cast `/Game/Blueprints/BP_GameInstance` (`GameplayStatics.GetGameInstance`)))
  (`/Game/Blueprints/BP_GameInstance.SetBoard` _asbp_game_instance self)
  (set `self.BoardDimensions` (0.0 0.0))
  (`self.BuildBoard` (0.0 0.0 0.0) (`self.Size_X`) (`self.Size_Y`))
  (for _array_element (`self.BoardTileset`)
    (`self.FillAdjacencyArray` _array_element (`/Game/Blueprints/BP_Tile.AdjacentTiles` _array_element)))
  (bind _returnvalue (`|SpawnActorFromClass` "/Game/Blueprints/BP_ObjectSpawner.BP_ObjectSpawner_C" (`KismetMathLibrary.MakeTransform` (0.0 0.0 0.0)) "Undefined" "MultiplyWithRoot" null null))
  (`/Game/Blueprints/BP_ObjectSpawner.SpawnObjects` _returnvalue))

(fn `BuildBoard`
  (params (Center :type "Vector Structure") (X :type Integer) (Y :type Integer))
  (locals (TileSize :type "Float (double-precision)" :default 100.0) (SpawnLocation :type "Vector Structure"))
  (if (== (`KismetArrayLibrary.Array_Length` (`self.BoardTileset`)) 0)
    (set `self.BoardDimensions` (`KismetMathLibrary.MakeVector2D` (`KismetMathLibrary.Conv_IntToDouble` X) (`KismetMathLibrary.Conv_IntToDouble` Y)))
    (for _index (range Y)
      (for _index_2 (range X)
        (bind _output_get (set `local.SpawnLocation` (`KismetMathLibrary.MakeVector` (- _index_2 (/ (`local.X`) 2)) (- _index (/ (`self.Size_Y`) 2)))))
        (castclass `/Game/Blueprints/BP_Tile` "/Game/Blueprints/BP_Tile.BP_Tile_C")
        (bind _returnvalue (`|SpawnActorFromClass` "/Game/Blueprints/BP_Tile.BP_Tile_C" (`KismetMathLibrary.MakeTransform` (+ (* (* _output_get (`local.TileSize`)) 1.0) (`local.Center`))) "Undefined" "MultiplyWithRoot" null null))
        (set `/Game/Blueprints/BP_Tile.Tile Info` (make `/Game/Blueprints/Structures/S_TileInfo` _output_get) _returnvalue)
        (`KismetArrayLibrary.Array_Add` (`self.BoardTileset`) _returnvalue)
        (`self.K2_AttachToActor` _returnvalue self "None" "KeepRelative" "KeepRelative" "KeepRelative" true)))))

(fn `FillAdjacencyArray`
  (params (CurrentTile :type "/Game/Blueprints/BP_Tile Object Reference") (TargetArray :type "Array of /Game/Blueprints/BP_Tile Object Reference"))
  (bind _currenttile (`local.CurrentTile`))
  (bind _currenttile_2 (`local.CurrentTile`))
  (bind _currenttile_3 (`local.CurrentTile`))
  (bind _currenttile_4 (`local.CurrentTile`))
  (bind _currenttile_5 (`local.CurrentTile`))
  (bind _currenttile_6 (`local.CurrentTile`))
  (bind _currenttile_7 (`local.CurrentTile`))
  (bind _currenttile_8 (`local.CurrentTile`))
  (bind _targetarray (`local.TargetArray`))
  (bind _returnvalue (`self.K2_GetActorLocation` _currenttile))
  (bind _returnvalue_2 (`self.K2_GetActorLocation` _currenttile_5))
  (bind _returnvalue_3 (`self.K2_GetActorLocation` _currenttile_6))
  (bind _returnvalue_4 (`self.K2_GetActorLocation` _currenttile_7))
  (bind _returnvalue_5 (`self.K2_GetActorLocation` _currenttile_8))
  (bind _returnvalue_6 (`self.K2_GetActorLocation` _currenttile_2))
  (bind _returnvalue_7 (`self.K2_GetActorLocation` _currenttile_3))
  (bind _returnvalue_8 (`self.K2_GetActorLocation` _currenttile_4))
  (`|ExecutionSequence`
    (:`then_0`
      (bind _adjacenttile (`self.HitTiles` _returnvalue_2 (+ _returnvalue_2 (100.0 0.0 0.0)) _currenttile_5)))
    (:`then_1`
      (bind _adjacenttile_2 (`self.HitTiles` _returnvalue_3 (+ _returnvalue_3 (-100.0 0.0 0.0)) _currenttile_6)))
    (:`then_2`
      (bind _adjacenttile_3 (`self.HitTiles` _returnvalue_4 (+ _returnvalue_4 (0.0 100.0 0.0)) _currenttile_7)))
    (:`then_3`
      (bind _adjacenttile_4 (`self.HitTiles` _returnvalue_5 (+ _returnvalue_5 (0.0 -100.0 0.0)) _currenttile_8)))
    (:`then_4`
      (bind _adjacenttile_5 (`self.HitTiles` _returnvalue_7 (+ _returnvalue_7 (100.0 100.0 0.0)) _currenttile_3)))
    (:`then_5`
      (bind _adjacenttile_6 (`self.HitTiles` _returnvalue_8 (+ _returnvalue_8 (-100.0 -100.0 0.0)) _currenttile_4)))
    (:`then_6`
      (bind _adjacenttile_7 (`self.HitTiles` _returnvalue_6 (+ _returnvalue_6 (-100.0 100.0 0.0)) _currenttile_2)))
    (:`then_7`
      (bind _adjacenttile_8 (`self.HitTiles` _returnvalue (+ _returnvalue (100.0 -100.0 0.0)) _currenttile)))
    (:`then_8`
      (`KismetArrayLibrary.Array_AddUnique` _targetarray _adjacenttile)
      (`KismetArrayLibrary.Array_AddUnique` _targetarray _adjacenttile_2)
      (`KismetArrayLibrary.Array_AddUnique` _targetarray _adjacenttile_3)
      (`KismetArrayLibrary.Array_AddUnique` _targetarray _adjacenttile_4)
      (`KismetArrayLibrary.Array_AddUnique` _targetarray _adjacenttile_5)
      (`KismetArrayLibrary.Array_AddUnique` _targetarray _adjacenttile_6)
      (`KismetArrayLibrary.Array_AddUnique` _targetarray _adjacenttile_7)
      (`KismetArrayLibrary.Array_AddUnique` _targetarray _adjacenttile_8))))

(fn `HitTiles`
  (params (Start :type "Vector Structure") (End :type "Vector Structure") (Emitter :type "/Game/Blueprints/BP_Tile Object Reference"))
  (returns (AdjacentTile :type "/Game/Blueprints/BP_Tile Object Reference"))
  (bind _outhit (`KismetSystemLibrary.LineTraceSingle` Start End "TraceTypeQuery1" false (`|MakeArray` Emitter :!type "Actor Object Reference") "None" true (struct :`R` 1.0 :`A` 1.0) (struct :`G` 1.0 :`A` 1.0) 0.0))
  (bind _asbp_tile (cast `/Game/Blueprints/BP_Tile` (`.HitActor` (`GameplayStatics.BreakHitResult` _outhit))))
  (return _asbp_tile))

(fn `PopulateAdjacentTiles`
  (params (A :type Integer) (X :type Integer))
  (returns (Array :type "Array of /Game/Blueprints/BP_Tile Object Reference"))
  (bind _boardtileset (`self.BoardTileset`))
  (return (`|MakeArray` (`|GetArrayItem` _boardtileset (+ A 1)) (`|GetArrayItem` _boardtileset (- A 1)) (`|GetArrayItem` _boardtileset (- A X)) (`|GetArrayItem` _boardtileset (- A X 1)) (`|GetArrayItem` _boardtileset (- A X -1)) (`|GetArrayItem` _boardtileset (+ A X)) (`|GetArrayItem` _boardtileset (+ A X -1)) (`|GetArrayItem` _boardtileset (+ A X 1)))))

(fn `UserConstructionScript`)