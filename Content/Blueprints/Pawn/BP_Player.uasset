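; BP_Player is the player controller Blueprint for a tile board game, handling mouse-driven piece movement.
; On BeginPlay it shows the cursor and spawns a BP_Pawn on a random tile from the game instance's board.
; Pressing selects a pawn and switches the cursor trace to WorldStatic; releasing over an adjacent tile moves it and restores pawn tracing.
; Tick prints the hovered actor and PointCount for debugging.
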(event `self.ReceiveBeginPlay`
  (bind (_returnvalue_x _returnvalue_y) (`KismetMathLibrary.BreakVector` (`self.K2_GetActorLocation` (`self.TileSpawn`))))
  (set `PlayerController.bShowMouseCursor` true (`GameplayStatics.GetPlayerController` 0))
  (bind _asbp_game_instance (cast `/Game/Blueprints/BP_GameInstance` (`GameplayStatics.GetGameInstance`)))
  (set `self.TileSpawn` (`KismetArrayLibrary.Array_Random` (`/Game/Blueprints/BP_TIleMap.BoardTileset` (`/Game/Blueprints/BP_GameInstance.BoardObject` _asbp_game_instance))))
  (bind _returnvalue (`|SpawnActorFromClass` "/Game/Blueprints/Pawn/BP_Pawn.BP_Pawn_C" (`KismetMathLibrary.MakeTransform` (`KismetMathLibrary.MakeVector` _returnvalue_x _returnvalue_y 70.0)) "Undefined" "MultiplyWithRoot" null null))
  (set `/Game/Blueprints/Pawn/BP_Pawn.TileLocation` (`self.TileSpawn`) _returnvalue))

(event `self.ReceiveTick`
  (params (DeltaSeconds :type "Float (single-precision)"))
  (`KismetSystemLibrary.PrintString` (`KismetSystemLibrary.GetDisplayName` (`.HitActor` (`GameplayStatics.BreakHitResult` (`PlayerController.GetHitResultUnderCursorForObjects` (`GameplayStatics.GetPlayerController` 0) (`|MakeArray` (`self.QueryType`)) true)))) true true (struct :`R` 1.0 :`B` 0.427554 :`A` 1.0) 0.0)
  (`KismetSystemLibrary.PrintString` (`KismetStringLibrary.Conv_IntToString` (`self.PointCount`)) true true (struct :`G` 1.0 :`B` 0.025953 :`A` 1.0) 0.0))

(event `Key|LeftMouseButton`
  (params (Key :type "Key Structure"))
  (bind _pawn (`self.Pawn`))
  (bind (_bblockinghit _binitialoverlap _time _distance _location _impactpoint _normal _impactnormal _physmat _hitactor) (`GameplayStatics.BreakHitResult` (`PlayerController.GetHitResultUnderCursorForObjects` (`GameplayStatics.GetPlayerController` 0) (`|MakeArray` (`self.QueryType`)) true)))
  (bind (_returnvalue_x _returnvalue_y) (`KismetMathLibrary.BreakVector` (`self.K2_GetActorLocation` _hitactor)))
  (:`Pressed`
    (bind _asbp_pawn (cast `/Game/Blueprints/Pawn/BP_Pawn` _hitactor))
    (bind _output_get (set `self.Pawn` _asbp_pawn))
    (`/Game/Blueprints/Pawn/BP_Pawn.OnSelected` _output_get)
    (set `self.QueryType` "ObjectTypeQuery1"))
  (:`Released`
    (bind _asbp_tile (cast `/Game/Blueprints/BP_Tile` _hitactor))
    (`/Engine/EditorBlueprintResources/StandardMacros.IsValid` _pawn
      (:`Is Valid`
        (`/Game/Blueprints/Pawn/BP_Pawn.OnUnselected` (`self.Pawn`))
        (if (`KismetArrayLibrary.Array_Contains` (`/Game/Blueprints/Pawn/BP_Pawn.AdjacentTileArray` _pawn) _asbp_tile)
          (`self.K2_SetActorLocation` (`self.Pawn`) (`KismetMathLibrary.MakeVector` _returnvalue_x _returnvalue_y 70.0) false false)
          (`/Game/Blueprints/Pawn/BP_Pawn.ClearAdjacentTileArray` (`self.Pawn`))
          (set `/Game/Blueprints/Pawn/BP_Pawn.TileLocation` _asbp_tile (`self.Pawn`))
          (set `self.QueryType` "ObjectTypeQuery3"))))))

(fn `UserConstructionScript`)