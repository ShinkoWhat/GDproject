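; Tile-board pawn that reveals items on neighbouring tiles and highlights those tiles when selected.
; Every Tick it line-traces from its TileLocation in four axis directions, changes neighbouring items' visibility and appends the hit tiles to AdjacentTileArray.
; Selection callbacks rescale the pawn and toggle the green material parameter on the array's first four entries.
; The array grows each frame, as ClearAdjacentTileArray is not called here, and Tick debug-prints the tile location.
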(event `self.ReceiveBeginPlay`
  (`|ExecutionSequence`
    (:`then_0`
      (add `self.OnSelected` (delegate `SelectedCallback`)))
    (:`then_1`
      (add `self.OnUnselected` (delegate `UnselectedCallback`)))))

(event `SelectedCallback`
  (`self.SetActorRelativeScale3D` (1.125 1.125 1.125))
  (`self.HighlightTiles`))

(event `UnselectedCallback`
  (`self.SetActorRelativeScale3D` (0.8 0.8 0.8))
  (`self.DropHighlight`))

(event `self.ReceiveTick`
  (params (DeltaSeconds :type "Float (single-precision)"))
  (bind _tilelocation (`self.TileLocation`))
  (`self.ExposeItems` _tilelocation)
  (`KismetSystemLibrary.PrintString` (`KismetStringLibrary.Conv_VectorToString` (`self.K2_GetActorLocation` _tilelocation)) true true (struct :`G` 0.66 :`B` 1.0 :`A` 1.0) 0.0))

(fn `ClearAdjacentTileArray`
  (`KismetArrayLibrary.Array_Clear` (`self.AdjacentTileArray`)))

(fn `DropHighlight`
  (bind _adjacenttilearray (`self.AdjacentTileArray`))
  (bind _output (`|GetArrayItem` _adjacenttilearray 3))
  (bind _output_2 (`|GetArrayItem` _adjacenttilearray))
  (bind _output_3 (`|GetArrayItem` _adjacenttilearray 1))
  (bind _output_4 (`|GetArrayItem` _adjacenttilearray 2))
  (`|ExecutionSequence`
    (:`then_0`
      (`/Engine/EditorBlueprintResources/StandardMacros.IsValid` _output_2
        (:`Is Valid`
          (`MaterialInstanceDynamic.SetScalarParameterValue` (`/Game/Blueprints/BP_Tile.MaterialInstance` _output_2) "GreenP" 0.0))))
    (:`then_1`
      (`/Engine/EditorBlueprintResources/StandardMacros.IsValid` _output_3
        (:`Is Valid`
          (`MaterialInstanceDynamic.SetScalarParameterValue` (`/Game/Blueprints/BP_Tile.MaterialInstance` _output_3) "GreenP" 0.0))))
    (:`then_2`
      (`/Engine/EditorBlueprintResources/StandardMacros.IsValid` _output_4
        (:`Is Valid`
          (`MaterialInstanceDynamic.SetScalarParameterValue` (`/Game/Blueprints/BP_Tile.MaterialInstance` _output_4) "GreenP" 0.0))))
    (:`then_3`
      (`/Engine/EditorBlueprintResources/StandardMacros.IsValid` _output
        (:`Is Valid`
          (`MaterialInstanceDynamic.SetScalarParameterValue` (`/Game/Blueprints/BP_Tile.MaterialInstance` _output) "GreenP" 0.0))))))

(fn `ExposeItems`
  (params (CurrentTile :type "/Game/Blueprints/BP_Tile Object Reference"))
  (bind _adjacenttilearray (`self.AdjacentTileArray`))
  (bind _returnvalue (`self.K2_GetActorLocation` (`local.CurrentTile`)))
  (bind _returnvalue_2 (`self.K2_GetActorLocation` (`local.CurrentTile`)))
  (`|ExecutionSequence`
    (:`then_0`
      (bind _adjacenttile (`self.HitTiles` (`self.K2_GetActorLocation` (`local.CurrentTile`)) (+ _returnvalue_2 (100.0 0.0 0.0)))))
    (:`then_1`
      (bind _adjacenttile_2 (`self.HitTiles` (`self.K2_GetActorLocation` (`local.CurrentTile`)) (+ _returnvalue_2 (-100.0 0.0 0.0)))))
    (:`then_2`
      (bind _adjacenttile_3 (`self.HitTiles` (`self.K2_GetActorLocation` (`local.CurrentTile`)) (+ _returnvalue (0.0 100.0 0.0)))))
    (:`then_3`
      (bind _adjacenttile_4 (`self.HitTiles` (`self.K2_GetActorLocation` (`local.CurrentTile`)) (+ _returnvalue (0.0 -100.0 0.0)))))
    (:`then_4`
      (`KismetArrayLibrary.Array_Add` _adjacenttilearray _adjacenttile)
      (`KismetArrayLibrary.Array_Add` _adjacenttilearray _adjacenttile_2)
      (`KismetArrayLibrary.Array_Add` _adjacenttilearray _adjacenttile_3)
      (`KismetArrayLibrary.Array_Add` _adjacenttilearray _adjacenttile_4))))

(fn `HighlightTiles`
  (bind _adjacenttilearray (`self.AdjacentTileArray`))
  (bind _output (`|GetArrayItem` _adjacenttilearray 3))
  (bind _output_2 (`|GetArrayItem` _adjacenttilearray))
  (bind _output_3 (`|GetArrayItem` _adjacenttilearray 1))
  (bind _output_4 (`|GetArrayItem` _adjacenttilearray 2))
  (`|ExecutionSequence`
    (:`then_0`
      (`/Engine/EditorBlueprintResources/StandardMacros.IsValid` _output_2
        (:`Is Valid`
          (`MaterialInstanceDynamic.SetScalarParameterValue` (`/Game/Blueprints/BP_Tile.MaterialInstance` _output_2) "GreenP" 1.0))))
    (:`then_1`
      (`/Engine/EditorBlueprintResources/StandardMacros.IsValid` _output_3
        (:`Is Valid`
          (`MaterialInstanceDynamic.SetScalarParameterValue` (`/Game/Blueprints/BP_Tile.MaterialInstance` _output_3) "GreenP" 1.0))))
    (:`then_2`
      (`/Engine/EditorBlueprintResources/StandardMacros.IsValid` _output_4
        (:`Is Valid`
          (`MaterialInstanceDynamic.SetScalarParameterValue` (`/Game/Blueprints/BP_Tile.MaterialInstance` _output_4) "GreenP" 1.0))))
    (:`then_3`
      (`/Engine/EditorBlueprintResources/StandardMacros.IsValid` _output
        (:`Is Valid`
          (`MaterialInstanceDynamic.SetScalarParameterValue` (`/Game/Blueprints/BP_Tile.MaterialInstance` _output) "GreenP" 1.0))))))

(fn `HitTiles`
  (params (Start :type "Vector Structure") (End :type "Vector Structure"))
  (returns (AdjacentTile :type "/Game/Blueprints/BP_Tile Object Reference"))
  (bind _outhit (`KismetSystemLibrary.LineTraceSingle` Start End "TraceTypeQuery1" false (`|MakeArray` (`self.TileLocation`) :!type "Actor Object Reference") "None" true (struct :`R` 1.0 :`A` 1.0) (struct :`G` 1.0 :`A` 1.0) 0.0))
  (bind _asbp_tile (cast `/Game/Blueprints/BP_Tile` (`.HitActor` (`GameplayStatics.BreakHitResult` _outhit))))
  (`|ExecutionSequence`
    (:`then_0`
      (bind _tileitem (`/Game/Blueprints/BP_Tile.TileItem` _asbp_tile)
        (:`then`
          (`/Game/Items/BP_BaseItem.SetVisibility` _tileitem "NewEnumerator1"))
        (:`else`)))
    (:`then_1`
      (return _asbp_tile))))

(fn `UserConstructionScript`)