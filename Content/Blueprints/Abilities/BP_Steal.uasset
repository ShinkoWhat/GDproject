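; BP_Steal is an ability named "Steal" that takes up to three points from another player in a tile-based game.
; Its Ability override runs the parent logic, then casts the hit actor to BP_Tile to find the player standing on it.
; If that player is valid and not the user's own pawn, it transfers the points, clamping the victim at zero.
; A successful steal ends the user's turn.
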(event `self.ReceiveBeginPlay`
  (`parent.ReceiveBeginPlay`)
  (set `self.Name` "Steal"))

(fn `Ability`
  (bind _parentplayer (`self.ParentPlayer`))
  (bind _pointcount (`/Game/Blueprints/Pawn/BP_Player.PointCount` _parentplayer))
  (`parent.Ability`)
  (bind _asbp_tile (cast `/Game/Blueprints/BP_Tile` (`self.ActorHitResult`)))
  (bind _playerontile (`/Game/Blueprints/BP_Tile.PlayerOnTile` _asbp_tile)
    (:`then`
      (if (!= _playerontile (`/Game/Blueprints/Pawn/BP_Player.Pawn` _parentplayer))
        (bind _playerpawn (`/Game/Blueprints/Pawn/BP_Pawn.PlayerPawn` _playerontile))
        (bind _pointcount_2 (`/Game/Blueprints/Pawn/BP_Player.PointCount` _playerpawn))
        (bind _returnvalue (- _pointcount_2 3))
        (if (> _returnvalue 0)
          (set `/Game/Blueprints/Pawn/BP_Player.PointCount` _returnvalue _playerpawn)
          (set `/Game/Blueprints/Pawn/BP_Player.PointCount` (+ _pointcount 3) _parentplayer)
          (`/Game/Blueprints/Pawn/BP_Player.OnTurnEnd` _parentplayer)
          (else
            (set `/Game/Blueprints/Pawn/BP_Player.PointCount` (+ _pointcount _pointcount_2) _parentplayer)
            (set `/Game/Blueprints/Pawn/BP_Player.PointCount` 0 _playerpawn)
            (`/Game/Blueprints/Pawn/BP_Player.OnTurnEnd` _parentplayer)))))
    (:`else`)))

(fn `UserConstructionScript`
  (`parent.UserConstructionScript`))