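; BP_Scan is a player ability named "Scan" that changes the visibility state of items on nearby tiles, likely revealing them.
; It overrides the parent's Ability function, walking neighbors of the tiles adjacent to the player pawn's tile through nested loops.
; Each valid tile item found gets its visibility set and triggers the player's turn-end call inside the loop, so finding none leaves the turn running.
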(event `self.ReceiveBeginPlay`
  (`parent.ReceiveBeginPlay`)
  (set `self.Name` "Scan"))

(fn `Ability`
  (`parent.Ability`)
  (for _array_element (`/Game/Blueprints/BP_Tile.AdjacentTiles` (`/Game/Blueprints/Pawn/BP_Pawn.TileLocation` (`/Game/Blueprints/Pawn/BP_Player.Pawn` (`self.ParentPlayer`))))
    (`/Engine/EditorBlueprintResources/StandardMacros.IsValid` _array_element
      (:`Is Valid`
        (for _array_element_2 (`/Game/Blueprints/BP_Tile.AdjacentTiles` _array_element)
          (bind _tileitem (`/Game/Blueprints/BP_Tile.TileItem` _array_element_2)
            (:`then`
              (`/Game/Items/BP_BaseItem.SetVisibility` _tileitem "NewEnumerator1")
              (`/Game/Blueprints/Pawn/BP_Player.OnTurnEnd` (`self.ParentPlayer`)))
            (:`else`)))))))

(fn `UserConstructionScript`
  (`parent.UserConstructionScript`))