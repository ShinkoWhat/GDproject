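; BP_PlaceMine is the "Place Mine" ability, which puts a land mine on a targeted tile in a turn-based game.
; Its Ability override casts the hit actor to BP_Tile and spawns a BP_LandMine above that tile's location at a fixed height.
; It sets the mine's turn countdown and visibility and triggers the owning player's turn end.
; Only after that turn-end call does it link the mine to the tile and activate it.
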(event `self.ReceiveBeginPlay`
  (`parent.ReceiveBeginPlay`)
  (set `self.Name` "Place Mine"))

(fn `Ability`
  (`parent.Ability`)
  (bind _asbp_tile (cast `/Game/Blueprints/BP_Tile` (`self.ActorHitResult`)))
  (bind (_returnvalue_x _returnvalue_y) (`KismetMathLibrary.BreakVector` (`self.K2_GetActorLocation` _asbp_tile)))
  (bind _returnvalue (`|SpawnActorFromClass` "/Game/Items/BP_LandMine.BP_LandMine_C" (`KismetMathLibrary.MakeTransform` (`KismetMathLibrary.MakeVector` _returnvalue_x _returnvalue_y 50.0)) "AlwaysSpawn" "MultiplyWithRoot" null null))
  (set `/Game/Items/BP_LandMine.TurnTickCount` 4 _returnvalue)
  (`/Game/Items/BP_BaseItem.SetVisibility` _returnvalue "NewEnumerator1")
  (`/Game/Blueprints/Pawn/BP_Player.OnTurnEnd` (`self.ParentPlayer`))
  (set `/Game/Items/BP_BaseItem.Tile` _asbp_tile _returnvalue)
  (`/Game/Items/BP_LandMine.ActivateMine` _returnvalue))

(fn `UserConstructionScript`
  (`parent.UserConstructionScript`))