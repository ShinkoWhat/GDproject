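; Object spawner actor that scatters items of a configured class across random tiles of the game board.
; On BeginPlay it takes the board from BP_GameInstance and calls its CallOnBoardSpawn; SpawnObjects separately runs RandomSpawn for about half the tile count.
; Each spawn sits at a fixed height over its tile, which stores the item, changes state and passes that state to the item's visibility.
; Tile picks can repeat, overwriting the stored item.
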(event `self.ReceiveBeginPlay`
  (bind _asbp_game_instance (cast `/Game/Blueprints/BP_GameInstance` (`GameplayStatics.GetGameInstance`)))
  (bind _output_get (set `self.BoardObject` (`/Game/Blueprints/BP_GameInstance.BoardObject` _asbp_game_instance)))
  (`/Game/Blueprints/BP_TIleMap.OnBoardSpawn` _output_get))

(event `SpawnObjects`
  (`self.RandomSpawn` (`self.ItemRef`) (/ (`KismetArrayLibrary.Array_Length` (`/Game/Blueprints/BP_TIleMap.BoardTileset` (`self.BoardObject`))) 2)))

(fn `RandomSpawn`
  (params (ClassArray :type "/Game/Items/BP_BaseItem Class Reference") (Amount :type Integer))
  (locals (TileInstance :type "/Game/Blueprints/BP_Tile Object Reference"))
  (bind (_returnvalue_x _returnvalue_y) (`KismetMathLibrary.BreakVector` (`self.K2_GetActorLocation` (`local.TileInstance`))))
  (for _ (range (+ Amount 1))
    (set `local.TileInstance` (`KismetArrayLibrary.Array_Random` (`/Game/Blueprints/BP_TIleMap.BoardTileset` (`self.BoardObject`))))
    (bind _returnvalue (`|SpawnActorFromClass` ClassArray (`KismetMathLibrary.MakeTransform` (`KismetMathLibrary.MakeVector` _returnvalue_x _returnvalue_y 50.0)) "Undefined" "MultiplyWithRoot" null null))
    (set `/Game/Blueprints/BP_Tile.TileItem` _returnvalue (`local.TileInstance`))
    (bind _output_get (set `/Game/Blueprints/BP_Tile.TileState` "NewEnumerator3" (`local.TileInstance`)))
    (`/Game/Items/BP_BaseItem.SetVisibility` _returnvalue _output_get)))

(fn `UserConstructionScript`)