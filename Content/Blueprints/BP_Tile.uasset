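; BP_Tile is a platform tile actor that knows its grid coordinates and detects a pawn standing on it.
; On BeginPlay it creates a dynamic material instance for its mesh and derives integer X, Y, Z indices from TileInfo coordinates divided by 100.
; Each Tick it line-traces a short distance upward and stores any BP_Pawn hit as PlayerOnTile, which is never cleared here.
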(event `self.ReceiveBeginPlay`
  (bind _tile_info (`self.Tile Info`))
  (bind _returnvalue (`PrimitiveComponent.CreateDynamicMaterialInstance` (`self.Tile1`) 0 "/Game/Materials/M_TilePlatform.M_TilePlatform" "None"))
  (set `self.MaterialInstance` _returnvalue)
  (set `self.Xi` (`KismetMathLibrary.FTrunc` (/ (.x (break `/Game/Blueprints/Structures/S_TileInfo` _tile_info)) 100.0)))
  (set `self.Yi` (`KismetMathLibrary.FTrunc` (/ (.y (break `/Game/Blueprints/Structures/S_TileInfo` _tile_info)) 100.0)))
  (set `self.Zi` (`KismetMathLibrary.FTrunc` (/ (.z (break `/Game/Blueprints/Structures/S_TileInfo` _tile_info)) 100.0))))

(event `self.ReceiveTick`
  (params (DeltaSeconds :type "Float (single-precision)"))
  (bind _returnvalue (`self.K2_GetActorLocation`))
  (bind _outhit (`KismetSystemLibrary.LineTraceSingle` _returnvalue (+ _returnvalue (0.0 0.0 100.0)) "TraceTypeQuery1"))
  (bind _asbp_pawn (cast `/Game/Blueprints/Pawn/BP_Pawn` (`.HitActor` (`GameplayStatics.BreakHitResult` _outhit))))
  (set `self.PlayerOnTile` _asbp_pawn))

(fn `UserConstructionScript`)