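; BP_CardPool is a player's hand of cards in a board game, expecting BP_Player as its owner.
; It fills an opening hand on BeginPlay by drawing random card instances from the GameModeBoard's deck controller, removing each from the shared deck and setting its parent player.
; Buying draws another card while under capacity, and using a card removes it from the hand and destroys its actor.
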(event `self.ReceiveBeginPlay`
  (for _ (range 5)
    (`self.DrawCardFromDeck`)))

(fn `BuyCard`
  (if (< (`KismetArrayLibrary.Array_Length` (`self.Cards`)) (`self.Capacity`))
    (`self.DrawCardFromDeck`)))

(fn `DrawCardFromDeck`
  (locals (RandomCardInstance :type "/Game/Blueprints/Abilities/BP_BaseAbility Object Reference"))
  (bind _asgame_mode_board (cast `/Game/Blueprints/GameModeBoard` (`GameplayStatics.GetGameMode`)))
  (bind _instantiatedcards (`/Game/Blueprints/BP_DeckController.InstantiatedCards` (`/Game/Blueprints/GameModeBoard.BP_DeckController` _asgame_mode_board)))
  (bind _output_get (set `local.RandomCardInstance` (`KismetArrayLibrary.Array_Random` _instantiatedcards)))
  (`KismetArrayLibrary.Array_Add` (`self.Cards`) _output_get)
  (bind _asbp_player (cast `/Game/Blueprints/Pawn/BP_Player` (`self.GetOwner`)))
  (set `/Game/Blueprints/Abilities/BP_BaseAbility.ParentPlayer` _asbp_player _output_get)
  (`KismetArrayLibrary.Array_RemoveItem` _instantiatedcards _output_get))

(fn `UseCard`
  (params (ChosenAbility :type "/Game/Blueprints/Abilities/BP_BaseAbility Object Reference"))
  (`KismetArrayLibrary.Array_RemoveItem` (`self.Cards`) ChosenAbility)
  (`Actor.K2_DestroyActor` ChosenAbility))