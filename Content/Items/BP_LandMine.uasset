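; BP_LandMine is a tile item for a turn-based board game that explodes after a countdown once noticed.
; Its OnNoticed event subscribes TickDown to the board game mode's OnNextTurn, lowering TurnTickCount each turn.
; At zero it removes players on adjacent tiles from the game, ends their turns, destroys them and items sharing their tiles, then destroys itself.
; A widget component receives a mine reference at BeginPlay.
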(event `self.ReceiveBeginPlay`
  (`parent.ReceiveBeginPlay`)
  (add `self.OnNoticed` (delegate `ActivateMine`))
  (bind _aswbp_land_mine_tick (cast `/Game/UI/WBP_LandMineTick` (`WidgetComponent.GetUserWidgetObject` (`self.Widget`))))
  (set `/Game/UI/WBP_LandMineTick.MineRef` self _aswbp_land_mine_tick))

(event `ActivateMine`
  (`|ExecutionSequence`
    (:`then_1`
      (bind _asgame_mode_board (cast `/Game/Blueprints/GameModeBoard` (`GameplayStatics.GetGameMode`)))
      (add `/Game/Blueprints/GameModeBoard.OnNextTurn` _asgame_mode_board (delegate `TickDown`)))))

(event `self.ReceiveTick`
  (params (DeltaSeconds :type "Float (single-precision)"))
  (`parent.ReceiveTick` DeltaSeconds))

(event `TickDown`
  (if (== (`self.TurnTickCount`) 0)
    (for _array_element (`/Game/Blueprints/BP_Tile.AdjacentTiles` (`self.Tile`))
      (bind _playerontile (`/Game/Blueprints/BP_Tile.PlayerOnTile` _array_element)
        (:`then`
          (bind _asgame_mode_board (cast `/Game/Blueprints/GameModeBoard` (`GameplayStatics.GetGameMode`)))
          (`KismetArrayLibrary.Array_RemoveItem` (`/Game/Blueprints/GameModeBoard.Players` _asgame_mode_board) (`/Game/Blueprints/Pawn/BP_Pawn.PlayerPawn` _playerontile))
          (`/Game/Blueprints/Pawn/BP_Player.OnTurnEnd` (`/Game/Blueprints/Pawn/BP_Pawn.PlayerPawn` _playerontile))
          (`/Engine/EditorBlueprintResources/StandardMacros.IsValid` _playerontile
            (:`Is Valid`
              (`/Game/Blueprints/Pawn/BP_Pawn.OnDestroy` _playerontile)
              (bind _tileitem (`/Game/Blueprints/BP_Tile.TileItem` _array_element)
                (:`then`
                  (`self.OnDestroy` _tileitem))
                (:`else`)))))
        (:`else`)))
    (`KismetSystemLibrary.DelayUntilNextTick`)
    (`self.K2_DestroyActor`)
    (else
      (`/Engine/EditorBlueprintResources/StandardMacros.DecrementInt` (`self.TurnTickCount`)))))

(fn `UserConstructionScript`
  (`parent.UserConstructionScript`))